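; BP_VRButton_Shirt4 is a VR push button that puts the fourth shirt on the ThirdPersonCharacter.
; When a VRPawn overlaps its Box, the Button component moves down from its starting position and WearShirt04 is called on the first ThirdPersonCharacter found in the level.
; A debug "Hello" prints on each press.
; When the pawn's overlap ends, the button moves back to its starting position.
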(event `self.ReceiveBeginPlay`
  (set `self.Button_Start` (`SceneComponent.RelativeLocation` (`self.button`))))

(event `self.Box.OnComponentBeginOverlap`
  (params (OverlappedComponent :type "PrimitiveComponent Object Reference") (OtherActor :type "Actor Object Reference") (OtherComp :type "PrimitiveComponent Object Reference") (OtherBodyIndex :type Integer) (bFromSweep :type Boolean) (SweepResult :type "HitResult Structure (by ref)"))
  (cast `/Game/VRTemplate/Blueprints/VRPawn` OtherActor)
  (`KismetSystemLibrary.MoveComponentTo` (`self.button`) (- (`self.Button_Start`) (0.0 0.0 5.0)))
  (bind _outactors (`GameplayStatics.GetAllActorsOfClass` "/Game/ModernMalePack/Blueprints/ThirdPersonCharacter.ThirdPersonCharacter_C"))
  (`KismetSystemLibrary.PrintString` "Hello")
  (`/Game/ModernMalePack/Blueprints/ThirdPersonCharacter.Wear_Shirt_04` (`|GetArrayItem` _outactors)))

(event `self.Box.OnComponentEndOverlap`
  (params (OverlappedComponent :type "PrimitiveComponent Object Reference") (OtherActor :type "Actor Object Reference") (OtherComp :type "PrimitiveComponent Object Reference") (OtherBodyIndex :type Integer))
  (cast `/Game/VRTemplate/Blueprints/VRPawn` OtherActor)
  (`KismetSystemLibrary.MoveComponentTo` (`self.button`) (`self.Button_Start`)))

(fn `UserConstructionScript`)