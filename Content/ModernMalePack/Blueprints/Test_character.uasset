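; Test character for the ModernMalePack that switches modular clothing pieces across shirt, pants, hat and shoe slots.
; Each wear event toggles component visibility to show one piece and hide the others in its slot.
; BeginPlay applies a default outfit through wear calls.
; The events for shirts 03, 04 and 05 all show Shirt01, so those three shirts never become visible through them.
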(event `self.ReceiveBeginPlay`
  ;[1 1 1] BEgin Event
  (`self.Wear_Shirt_02`)
  (`self.Wear_Pants_01`)
  (`self.Wear_Shoe_01`)
  (`self.Wear_Hat_01`))

(event `Wear_Shirt_04`
  ;[1 1 1] Shirts
  (`SceneComponent.SetVisibility` (`self.Shirt_01`) true false)
  (`SceneComponent.SetVisibility` (`self.Shirt_02`) false false)
  (`SceneComponent.SetVisibility` (`self.Shirt_03`) false false)
  (`SceneComponent.SetVisibility` (`self.Shirt_04`) false false)
  (`SceneComponent.SetVisibility` (`self.Shirt_05`) false false))

(event `Wear_Shirt_03`
  ;[1 1 1] Shirts
  (`SceneComponent.SetVisibility` (`self.Shirt_01`) true false)
  (`SceneComponent.SetVisibility` (`self.Shirt_02`) false false)
  (`SceneComponent.SetVisibility` (`self.Shirt_03`) false false)
  (`SceneComponent.SetVisibility` (`self.Shirt_04`) false false)
  (`SceneComponent.SetVisibility` (`self.Shirt_05`) false false))

(event `Wear_Shirt_05`
  ;[1 1 1] Shirts
  (`SceneComponent.SetVisibility` (`self.Shirt_01`) true false)
  (`SceneComponent.SetVisibility` (`self.Shirt_02`) false false)
  (`SceneComponent.SetVisibility` (`self.Shirt_03`) false false)
  (`SceneComponent.SetVisibility` (`self.Shirt_04`) false false)
  (`SceneComponent.SetVisibility` (`self.Shirt_05`) false false))

(event `Wear_Shirt_01`
  ;[1 1 1] Shirts
  (`SceneComponent.SetVisibility` (`self.Shirt_01`) true false)
  (`SceneComponent.SetVisibility` (`self.Shirt_02`) false false)
  (`SceneComponent.SetVisibility` (`self.Shirt_03`) false false)
  (`SceneComponent.SetVisibility` (`self.Shirt_04`) false false)
  (`SceneComponent.SetVisibility` (`self.Shirt_05`) false false))

(event `Wear_Shirt_02`
  ;[1 1 1] Shirts
  (`SceneComponent.SetVisibility` (`self.Shirt_01`) false false)
  (`SceneComponent.SetVisibility` (`self.Shirt_02`) true false)
  (`SceneComponent.SetVisibility` (`self.Shirt_03`) false false)
  (`SceneComponent.SetVisibility` (`self.Shirt_04`) false false)
  (`SceneComponent.SetVisibility` (`self.Shirt_05`) false false))

(event `Wear_Pants_01`
  ;[1 1 1] Pants
  (`SceneComponent.SetVisibility` (`self.Pant_01`) true false)
  (`SceneComponent.SetVisibility` (`self.Pant_03`) false false)
  (`SceneComponent.SetVisibility` (`self.Pant_02`) false false)
  (`SceneComponent.SetVisibility` (`self.Pant_04`) false false)
  (`SceneComponent.SetVisibility` (`self.Pant_05`) false false))

(event `Wear_Pants_02`
  ;[1 1 1] Pants
  (`SceneComponent.SetVisibility` (`self.Pant_01`) false false)
  (`SceneComponent.SetVisibility` (`self.Pant_03`) false false)
  (`SceneComponent.SetVisibility` (`self.Pant_02`) true false)
  (`SceneComponent.SetVisibility` (`self.Pant_04`) false false)
  (`SceneComponent.SetVisibility` (`self.Pant_05`) false false))

(event `Wear_Pants_03`
  ;[1 1 1] Pants
  (`SceneComponent.SetVisibility` (`self.Pant_01`) false false)
  (`SceneComponent.SetVisibility` (`self.Pant_03`) true false)
  (`SceneComponent.SetVisibility` (`self.Pant_02`) false false)
  (`SceneComponent.SetVisibility` (`self.Pant_04`) false false)
  (`SceneComponent.SetVisibility` (`self.Pant_05`) false false))

(event `Wear_Pants_04`
  ;[1 1 1] Pants
  (`SceneComponent.SetVisibility` (`self.Pant_01`) false false)
  (`SceneComponent.SetVisibility` (`self.Pant_03`) false false)
  (`SceneComponent.SetVisibility` (`self.Pant_02`) false false)
  (`SceneComponent.SetVisibility` (`self.Pant_04`) true false)
  (`SceneComponent.SetVisibility` (`self.Pant_05`) false false))

(event `WearPant_05`
  ;[1 1 1] Pants
  (`SceneComponent.SetVisibility` (`self.Pant_01`) false false)
  (`SceneComponent.SetVisibility` (`self.Pant_02`) false false)
  (`SceneComponent.SetVisibility` (`self.Pant_03`) false false)
  (`SceneComponent.SetVisibility` (`self.Pant_04`) false false)
  (`SceneComponent.SetVisibility` (`self.Pant_05`) true false))

(event `Wear_Hat_01`
  ;[1 1 1] Hats
  (`SceneComponent.SetVisibility` (`self.Hat_01`) true false)
  (`SceneComponent.SetVisibility` (`self.Hat_02`) false false)
  (`SceneComponent.SetVisibility` (`self.Hat_03`) false false))

(event `Wear_Hat_02`
  ;[1 1 1] Hats
  (`SceneComponent.SetVisibility` (`self.Hat_01`) false false)
  (`SceneComponent.SetVisibility` (`self.Hat_02`) true false)
  (`SceneComponent.SetVisibility` (`self.Hat_03`) false false))

(event `Wear_Hat_03`
  ;[1 1 1] Hats
  (`SceneComponent.SetVisibility` (`self.Hat_01`) false false)
  (`SceneComponent.SetVisibility` (`self.Hat_02`) false false)
  (`SceneComponent.SetVisibility` (`self.Hat_03`) true false))

(event `Wear_Shoe_01`
  ;[1 1 1] Shoes
  (`SceneComponent.SetVisibility` (`self.Shoes_01`) true false)
  (`SceneComponent.SetVisibility` (`self.Shoes_02`) false false))

(event `Wear_Shoe_02`
  ;[1 1 1] Shoes
  (`SceneComponent.SetVisibility` (`self.Shoes_01`) false false)
  (`SceneComponent.SetVisibility` (`self.Shoes_02`) true false))

(fn `UserConstructionScript`)